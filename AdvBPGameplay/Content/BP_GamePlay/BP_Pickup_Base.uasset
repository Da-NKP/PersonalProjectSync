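; Base pickup Blueprint that spins in place and is collected when the player character touches it.
; Sphere overlap compares the other actor to the player character (index wired from OtherBodyIndex), reports PickupType to the GameMode, then destroys the pickup.
; Tick applies a frame-rate-independent local yaw spin scaled by Multiplier.
; The construction script assigns StaticMeshToDisplay to PickupMesh.
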(event `self.SphereCollider.OnComponentBeginOverlap`
  (params (OtherActor :type "Actor Object Reference") (OtherComp :type "PrimitiveComponent Object Reference") (OtherBodyIndex :type Integer) (bFromSweep :type Boolean) (SweepResult :type "HitResult Structure (by ref)"))
  ;[1 1 1] Player Collision
  (if (== (`GameplayStatics.GetPlayerCharacter` OtherBodyIndex) OtherActor)
    (message `/Game/BPI_Gameplay/BPI_GameMode.CollectedPickups` (`GameplayStatics.GetGameMode`) (`self.PickupType`))
    (`self.K2_DestroyActor`)))

(event `self.ReceiveTick`
  (params (DeltaSeconds :type "Float (single-precision)"))
  ;[1 1 1] Rotation
  (`self.K2_AddActorLocalRotation` (`KismetMathLibrary.MakeRotator` 0.0 0.0 (* DeltaSeconds (`self.Multiplier`)))))

(fn `UserConstructionScript`
  (`StaticMeshComponent.SetStaticMesh` (`self.PickupMesh`) (`self.StaticMeshToDisplay`)))